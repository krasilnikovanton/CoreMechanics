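; Base player character Blueprint with physics object carrying, crouching and an inventory view.
; A camera line trace grabs simulating components with a PhysicsHandle, whose target follows the scene camera through a per-frame Delay loop, and held objects drop or launch by impulse.
; A timeline drives capsule height and mesh offset for crouching.
; The Inventory input blends to an inventory camera and opens a UI-only widget with cursor.
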(event Custom|DROPOBJECT
  ;[1 1 1] Take and drop items
  (Physics|Components|PhysicsHandle|ReleaseComponent (Variables|Default|GetPhysicsHandle))
  (Variables|Default|SetisHoldingObject false)
  (Collision|SetCollisionResponsetoChannel (.HitComponent (Collision|BreakHitResult (stale Custom|PICK%20UP%20OBJECT _outhit))) "ECC_Pawn" "ECR_Block"))

(event Custom|PICK%20UP%20OBJECT
  (bind _cameracomponent (Variables|Default|GetCameraComponent))
  (bind _returnvalue (Transformation|GetWorldLocation _cameracomponent))
  ;[1 1 1] Take and drop items
  (bind (_outhit _returnvalue_2) (Collision|LineTraceByChannel _returnvalue (+ (* (Math|Vector|GetForwardVector _cameracomponent) 2e+02) _returnvalue) "TraceTypeQuery1" false 0 "ForDuration"))
  (if _returnvalue_2
    (if (Physics|IsSimulatingPhysics (.HitComponent (Collision|BreakHitResult _outhit)) "None")
      (Physics|Components|PhysicsHandle|GrabComponentatLocationwithRotation (Variables|Default|GetPhysicsHandle) (.HitComponent (Collision|BreakHitResult _outhit)) "None" (Transformation|GetWorldLocation (.HitComponent (Collision|BreakHitResult _outhit))) "0, 0, 0")
      (Variables|Default|SetisHoldingObject true)
      (Collision|SetCollisionResponsetoChannel (.HitComponent (Collision|BreakHitResult _outhit)) "ECC_Pawn" "ECR_Ignore"))))

(event EventPickUpInterp
  (params (isHolding :type Boolean))
  ;[1 1 1] Take and drop items
  (if isHolding
    (CallFunction|DROPOBJECT)
    (else
      (CallFunction|PICKUPOBJECT))))

(event EventBeginPlay
  (bind _scenecameracomponent (Variables|Default|GetSceneCameraComponent))
  ;[1 1 1] Take and drop items
  (Utilities|FlowControl|Delay (Utilities|Time|GetWorldDeltaSeconds) :!label _label)
  (Class|PhysicsHandleComponent|SetTargetLocationandRotation (Variables|Default|GetPhysicsHandle) (Transformation|GetWorldLocation _scenecameracomponent) (Transformation|GetWorldRotation _scenecameracomponent))
  (goto _label))

(event EventLaunchInterp
  (params (isHolding :type Boolean))
  ;[1 1 1] Take and drop items
  (if isHolding
    (CallFunction|DROPOBJECT)
    (Physics|AddImpulse (.HitComponent (Collision|BreakHitResult (stale Custom|PICK%20UP%20OBJECT _outhit))) (* (Math|Vector|GetForwardVector (Variables|Default|GetCameraComponent)) 2.4e+03) "None" true)))

(event EventCrouchInterp
  (params (IsCrouching :type Boolean))
  (bind _mesh (Variables|Character|GetMesh))
  (bind _relativelocation (Variables|/Script/Engine.SceneComponent|GetRelativeLocation _mesh))
  ;[1 1 1] Crouching
  (if IsCrouching
    (bind (_direction _capsuleheight _meshheight) (Timeline|CrouchTimeline Play)
      (:Update
        (Components|Capsule|SetCapsuleHalfHeight (Variables|Default|GetCapsuleComponent) _capsuleheight true)
        (Transformation|SetRelativeLocation _mesh (Math|Vector|MakeVector (.x _relativelocation) (.y _relativelocation) _meshheight) false false) ; Prevents the mesh failure bug
      ))
    (else
      (Timeline|CrouchTimeline Reverse))))

(event Input|ActionEvents|InputActionInventory
  (params (Key :type Key%20Structure :default "None"))
  (bind _returnvalue (Game|GetPlayerController 0))
  (:Pressed
    (Game|Player|SetViewTargetwithBlend (Game|GetPlayerController 0) (Variables|/Script/Engine.ChildActorComponent|GetChildActor (Variables|Default|GetInventoryCamera)) 0.5 "VTBlend_Linear" 0.0 false)
    (bind _returnvalue_2 (UserInterface|CreateWidget "/Game/UI/PlayerInventory_UI.PlayerInventory_UI_C" 0 0))
    (UserInterface|Viewport|AddtoViewport _returnvalue_2 0)
    (Input|SetInputModeUIOnly _returnvalue 0 "DoNotLock")
    (Variables|/Script/Engine.PlayerController|SetbShowMouseCursor _returnvalue true)))

(fn ConstructionScript)

(fn SpendMoney
  (params (Money :type Integer))
  (Variables|Default|Setmoney (- (Variables|Default|Getmoney) Money))
  (return 0))